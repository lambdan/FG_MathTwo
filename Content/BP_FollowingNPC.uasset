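; A following NPC that turns toward the first player character and moves toward it every tick.
; Each tick, an IsFaster check between itself and the player switches the max walk speed between a fast and a slow value, with true selecting the fast one.
; It then snaps its rotation to look at the player and adds forward movement input, steering directly without pathfinding.
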(event EventTick
  (params (DeltaSeconds :type Float%20%28single-precision%29))
  (bind _charactermovement (Variables|Character|GetCharacterMovement))
  (Utilities|FlowControl|Sequence
    (:then_0
      (if (Class|MathLibrary|IsFaster self (Game|GetPlayerCharacter 0))
        (Variables|/Script/Engine.CharacterMovementComponent|SetMaxWalkSpeed _charactermovement 5e+02)
        (else
          (Variables|/Script/Engine.CharacterMovementComponent|SetMaxWalkSpeed _charactermovement 2.5e+02))))
    (:then_1
      (Transformation|SetActorRotation (Math|Rotator|FindLookatRotation (Transformation|GetActorLocation) (Transformation|GetActorLocation (Game|GetPlayerCharacter 0)))))
    (:then_2
      (Pawn|Input|AddMovementInput (Transformation|GetActorForwardVector) 1.0 false))))

(fn ConstructionScript)