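; BP_Enemy is a stealth-game enemy that rotates in place, spots the player and can be stealth killed.
; Each Tick it turns slightly, then runs an IsInFront facing check against player character 0, with no line trace in this graph.
; Detection shows exclamation text and plays an alert sound once per sighting, resetting when the player leaves its front.
; The StealthKill event prints a message and destroys the actor once.
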(event Custom|Detect%20player
  (if (Class|MathLibrary|IsinFront self (Game|GetPlayerCharacter 0) 0.9)
    (Development|PrintString "i see you" true true "(R=0.000000,G=0.660000,B=1.000000,A=1.000000)" 0.1 "icu")
    (Utilities|FlowControl|DoOnce false :!label _label
      (:Completed
        (Rendering|SetVisibility (Variables|Default|GetExclamationText) true false)
        (Audio|PlaySoundatLocation "/Game/Sound/mgs_alert.mgs_alert" (Transformation|GetActorLocation) "0, 0, 0" 1.0 1.0 0.0 0 0 0 0)))
    (else
      (Utilities|FlowControl|Sequence
        (:then_0
          (goto _label Reset))
        (:then_1
          (Rendering|SetVisibility (Variables|Default|GetExclamationText) false false))))))

(event EventTick
  (params (DeltaSeconds :type Float%20%28single-precision%29))
  (Class|Actor|AddActorWorldRotation "0.000000,0.300000,0.000000")
  (CallFunction|DetectPlayer))

(event EventStealthKill
  (Utilities|FlowControl|DoOnce false
    (:Completed
      (Development|PrintString "OH NO i got stealth killed")
      (Actor|DestroyActor))))

(fn ConstructionScript)