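; BP_IntersectionTest is a test actor that switches its point light on while it intersects the player character and off when it does not.
; Tick runs an AABBIntersection check between the actor and player character 0 instead of using overlap events.
; Two DoOnce gates reset each other, so the light's visibility is set only when the intersection state changes.
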(event EventBeginPlay)

(event Collision|EventActorBeginOverlap
  (params (OtherActor :type Actor%20Object%20Reference)))

(event EventTick
  (params (DeltaSeconds :type Float%20%28single-precision%29))
  (bind _pointlight (Variables|Default|GetPointLight))
  (if (Class|IntersectionLibrary|AABBIntersection self (Game|GetPlayerCharacter 0))
    (Utilities|FlowControl|Sequence
      (:then_0
        (goto _label_2 Reset))
      (:then_1
        (Utilities|FlowControl|DoOnce false :!label _label
          (:Completed
            (Rendering|SetVisibility _pointlight true false)))))
    (else
      (Utilities|FlowControl|Sequence
        (:then_0
          (goto _label Reset))
        (:then_1
          (Utilities|FlowControl|DoOnce false :!label _label_2
            (:Completed
              (Rendering|SetVisibility _pointlight false false))))))))

(fn ConstructionScript)